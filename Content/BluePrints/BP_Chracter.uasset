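; Player character Blueprint that handles camera-relative movement, look input and hitscan shooting at monsters.
; Movement follows control yaw and stores axis values in X and Y.
; The 1 key and Trigger action share one path that sets fire or reload flags from the bullet count.
; That path then line-traces from the camera regardless of ammo, destroying any BP_Monster hit and printing a debug string on a miss.
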(event `self.ReceiveBeginPlay`)

(event `self.ReceiveTick`
  (params (DeltaSeconds :type "Float (single-precision)")))

(event `InputAxis|MoveForword`
  (params (AxisValue :type "Float (single-precision)"))
  (`self.AddMovementInput` (`KismetMathLibrary.GetForwardVector` (`KismetMathLibrary.MakeRotator` 0.0 0.0 (.yaw (`self.GetControlRotation`)))) AxisValue)
  (set `self.x` AxisValue))

(event `InputAxis|MoveRight`
  (params (AxisValue :type "Float (single-precision)"))
  (`self.AddMovementInput` (`KismetMathLibrary.GetRightVector` (`KismetMathLibrary.MakeRotator` 0.0 0.0 (.yaw (`self.GetControlRotation`)))) AxisValue)
  (set `self.y` AxisValue))

(event `InputAxis|Turn`
  (params (AxisValue :type "Float (single-precision)"))
  (`self.AddControllerYawInput` AxisValue))

(event `InputAxis|LookUp`
  (params (AxisValue :type "Float (single-precision)"))
  (`self.AddControllerPitchInput` AxisValue))

(event `Key|One`
  (params (Key :type "Key Structure" :default "AnyKey"))
  (bind _returnvalue (`GameplayStatics.GetPlayerCameraManager` 0))
  (bind _returnvalue_2 (`PlayerCameraManager.GetCameraLocation` _returnvalue))
  (:`Pressed`
    (`|ExecutionSequence` :!label _label
      (:`then_0`
        (if (<= (`self.BullenCnt`) 0)
          (set `self.Reload` true)
          (set `self.BReload` true)
          (else
            (set `self.Fire` true)
            (set `self.Shot` true))))
      (:`then_1`
        (bind (_outhit _returnvalue_3) (`KismetSystemLibrary.LineTraceSingle` _returnvalue_2 (+ _returnvalue_2 (* (`KismetMathLibrary.GetForwardVector` (`PlayerCameraManager.GetCameraRotation` _returnvalue)) 10000.0)) "TraceTypeQuery1"))
        (if _returnvalue_3
          (bind _asbp_monster (cast `/Game/BluePrints/BP_Monster` (`.HitActor` (`GameplayStatics.BreakHitResult` _outhit))))
          (`self.K2_DestroyActor` _asbp_monster)
          (else
            (`KismetSystemLibrary.PrintString` "Hello")))))))

(event `InputAction|Trigger`
  (params (Key :type "Key Structure" :default "AnyKey"))
  (:`Pressed`
    (goto _label)))

(fn `UserConstructionScript`)